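; Survival game mode Blueprint that announces each incoming wave to the player with an on-screen countdown.
; On BeginPlay it binds to the survival state-changed delegate and reacts only to the Wait Spawn New Wave state.
; That state creates a wave text widget in the viewport, labels it with the current wave count and starts its countdown using the spawn wait time.
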(event `self.ReceiveBeginPlay`
  (add `self.OnSurvivalGameModeStateChanged` (delegate `OnSurvivalGameModeStateChanged_Event`)))

(event `OnSurvivalGameModeStateChanged_Event` :!signature `self.OnSurvivalGameModeStateChanged`
  (params (CurrentState :type "EUGRC_SurvivalGameModeState Enum" :default "WaitSpawnNewWave"))
  (switch `EUGRC_SurvivalGameModeState` CurrentState
    (:`WaitSpawnNewWave`
      (`self.CreateWaveWidgetWithCountDown` (`|FormatText` "Wave {CurrentWaveCount} Coming In" (`self.CurrentWaveCount`)) (`self.SpawnNewWaveWaitTime`)))))

(fn `CreateWaveWidgetWithCountDown`
  (params (TextContentToDisplay :type Text) (InTotalCountDownTime :type "Float (double-precision)"))
  (bind _returnvalue (`|CreateWidget` "/Game/Game/Widgets/GameModeWidgets/WBP_WaveTextWithCountDown.WBP_WaveTextWithCountDown_C"))
  (`UserWidget.AddToViewport` _returnvalue 0)
  (`TextBlock.SetText` (`/Game/Game/Widgets/GameModeWidgets/WBP_WaveTextWithCountDown.TextBlock_WaveText` _returnvalue) (`local.TextContentToDisplay`))
  (`/Game/Game/Widgets/GameModeWidgets/WBP_WaveTextWithCountDown.StartCountDown` _returnvalue (`local.InTotalCountDownTime`)))

(fn `UserConstructionScript`)